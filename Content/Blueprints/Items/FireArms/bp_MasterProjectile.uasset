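; Master firearm projectile Blueprint that plays a configurable, attenuated sound at its location on spawn and resolves its impact on hit.
; Hits on an FPS_Character apply base damage, plus a velocity-scaled impulse if the struck component simulates physics.
; Any other hit leaves a short-lived decal aligned to the surface normal.
; The projectile destroys itself after every hit.
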(event `self.ReceiveBeginPlay`
  (`GameplayStatics.PlaySoundAtLocation` (`self.Sound`) (`self.K2_GetActorLocation`) (struct) (`self.Volume Multiplier`) (`self.Pitch Multiplier`) 0.0 "/Game/Sounds/SA_NaturalFalloff.SA_NaturalFalloff" null null null))

(event `self.ReceiveHit`
  (params (MyComp :type "PrimitiveComponent Object Reference") (Other :type "Actor Object Reference") (OtherComp :type "PrimitiveComponent Object Reference") (bSelfMoved :type Boolean) (HitLocation :type "Vector Structure") (HitNormal :type "Vector Structure") (NormalImpulse :type "Vector Structure") (Hit :type "HitResult Structure (by ref)"))
  (bind _size (`self.Size`))
  (bind _asfps_character (cast `/Game/Blueprints/Character/FPS_Character` Other)
    (:`then`
      (`GameplayStatics.ApplyDamage` _asfps_character (`self.Base Damage`) null self)
      (if (`SceneComponent.IsSimulatingPhysics` OtherComp "None")
        (`PrimitiveComponent.AddImpulseAtLocation` OtherComp (* (`self.GetVelocity`) 100.0) (`self.K2_GetActorLocation`) "None")
        (`self.K2_DestroyActor`)
        (else
          (`self.K2_DestroyActor` :!label _label))))
    (:`CastFailed`
      (`GameplayStatics.SpawnDecalAtLocation` "/Game/Materials/M_Decal_Master.M_Decal_Master" (`KismetMathLibrary.MakeVector` _size _size _size) HitLocation (`KismetMathLibrary.MakeRotFromX` HitNormal) 5.0)
      (goto _label))))

(fn `UserConstructionScript`)