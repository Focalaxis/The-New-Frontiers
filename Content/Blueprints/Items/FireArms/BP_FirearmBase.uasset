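; Base firearm actor that attaches to a character and fires projectiles.
; On BeginPlay it casts player character 0 to BP_EnemyAI_Base, snaps to that mesh's clavicle_l socket and binds an event to the character's OnUseItem dispatcher.
; Shoot spawns Bp_MasterProjectile from that socket, offset by ProjectileOffset rotated to the character's facing, using the character's rotation.
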(event `self.ReceiveActorBeginOverlap`
  (params (OtherActor :type "Actor Object Reference")))

(event `self.ReceiveBeginPlay`
  (bind _asbp_enemy_ai_base (cast `/Game/Blueprints/AI/EnemyAI/BP_EnemyAI_Base` (`GameplayStatics.GetPlayerCharacter` 0)))
  (set `self.BP Enemy AI Base ref` _asbp_enemy_ai_base)
  (`self.K2_AttachToComponent` self (`Character.Mesh` (`self.BP Enemy AI Base ref`)) "clavicle_l" "SnapToTarget" "SnapToTarget" "SnapToTarget" true)
  (add `/Game/Blueprints/AI/EnemyAI/BP_EnemyAI_Base.OnUseItem` (`self.BP Enemy AI Base ref`) (`|CreateDelegate` :!event `Shoot`)))

(event `Shoot`
  (bind _returnvalue (`self.K2_GetActorRotation` (`self.BP Enemy AI Base ref`)))
  (`|SpawnActorFromClass` "/Game/Blueprints/Items/FireArms/bp_MasterProjectile.bp_MasterProjectile_C" (`KismetMathLibrary.MakeTransform` (+ (`SceneComponent.GetSocketLocation` (`Character.Mesh` (`self.BP Enemy AI Base ref`)) "clavicle_l") (`KismetMathLibrary.GreaterGreater_VectorRotator` (`self.Projectile Offset`) _returnvalue)) _returnvalue) "AlwaysSpawn" "OverrideRootScale" null 1.0 1.0 null 0.34 null))

(fn `UserConstructionScript`)