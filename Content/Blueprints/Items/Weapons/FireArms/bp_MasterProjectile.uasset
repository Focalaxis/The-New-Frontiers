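; Base firearm projectile that plays a blaster sound at its location on spawn and deals damage on hit.
; On hit, a Sequence runs separate casts to BP_EnemyAI_Base and FPS_Character, applying damage and a velocity-scaled impulse if the hit component simulates physics.
; Each failed cast branches into a shared impact path that spawns a short-lived decal aligned to the surface normal and destroys the projectile.
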(event `self.ReceiveBeginPlay`
  ;[1 1 1] Plays Sound for blaster
  (`GameplayStatics.PlaySoundAtLocation` (`self.Sound`) (`self.K2_GetActorLocation`) (struct) (`self.Volume Multiplier`) (`self.Pitch Multiplier`) 0.0 "/Game/Sounds/SA_NaturalFalloff.SA_NaturalFalloff" null null null))

(event `self.ReceiveHit`
  (params (MyComp :type "PrimitiveComponent Object Reference") (Other :type "Actor Object Reference") (OtherComp :type "PrimitiveComponent Object Reference") (bSelfMoved :type Boolean) (HitLocation :type "Vector Structure") (HitNormal :type "Vector Structure") (NormalImpulse :type "Vector Structure") (Hit :type "HitResult Structure (by ref)"))
  (bind _returnvalue (`self.K2_GetActorLocation`))
  (bind _returnvalue_2 (`SceneComponent.IsSimulatingPhysics` OtherComp "None"))
  (bind _base_damage (`self.Base Damage`))
  (bind _size (`self.Size`))
  (bind _returnvalue_3 (* (`self.GetVelocity`) 100.0))
  ;[1 1 1] Deals damage to bp and creates decal
  (`|ExecutionSequence`
    (:`then_0`
      (bind _asbp_enemy_ai_base (cast `/Game/Blueprints/AI/EnemyAI/BP_EnemyAI_Base` Other)
        (:`then`
          (`GameplayStatics.ApplyDamage` _asbp_enemy_ai_base _base_damage)
          (if _returnvalue_2
            (`PrimitiveComponent.AddImpulseAtLocation` (`Character.CapsuleComponent` _asbp_enemy_ai_base) _returnvalue_3 _returnvalue "None")
            (`self.K2_DestroyActor`)))
        (:`CastFailed`
          (`GameplayStatics.SpawnDecalAtLocation` "/Game/Materials/M_Decal_Master.M_Decal_Master" (`KismetMathLibrary.MakeVector` _size _size _size) HitLocation (`KismetMathLibrary.MakeRotFromX` HitNormal) 5.0 :!label _label)
          (`self.K2_DestroyActor` :!label _label_2))))
    (:`then_1`
      (bind _asfps_character (cast `/Game/Blueprints/Character/FPS_Character` Other)
        (:`then`
          (`GameplayStatics.ApplyDamage` _asfps_character _base_damage null self)
          (if _returnvalue_2
            (`PrimitiveComponent.AddImpulseAtLocation` OtherComp _returnvalue_3 _returnvalue "None")
            (`self.K2_DestroyActor`)
            (else
              (goto _label_2))))
        (:`CastFailed`
          (goto _label))))))

(fn `UserConstructionScript`)