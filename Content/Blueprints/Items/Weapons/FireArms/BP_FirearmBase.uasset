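; Base firearm Blueprint that an FPS_Character picks up by overlap and that fires projectiles.
; On sphere overlap it snaps to the character's hand_r socket and binds an event to that character's OnUseItem dispatcher.
; Its Shoot event spawns a scaled Bp_MasterProjectile with fixed base damage, positioned from the Magazine socket plus a camera-rotated offset and aimed along player 0's camera rotation.
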(event `self.Sphere.OnComponentBeginOverlap`
  (params (OverlappedComponent :type "PrimitiveComponent Object Reference") (OtherActor :type "Actor Object Reference") (OtherComp :type "PrimitiveComponent Object Reference") (OtherBodyIndex :type Integer) (bFromSweep :type Boolean) (SweepResult :type "HitResult Structure (by ref)"))
  (bind _asfps_character (cast `/Game/Blueprints/Character/FPS_Character` OtherActor))
  (set `self.FPS Character Ref` _asfps_character)
  (`self.K2_AttachToComponent` self (`Character.Mesh` (`self.FPS Character Ref`)) "hand_r" "SnapToTarget" "SnapToTarget" "SnapToTarget" true)
  (add `/Game/Blueprints/Character/FPS_Character.OnUseItem` (`self.FPS Character Ref`) (`|CreateDelegate` :!event `Shoot`)))

(event `Shoot`
  (bind _returnvalue (`PlayerCameraManager.GetCameraRotation` (`GameplayStatics.GetPlayerCameraManager` 0)))
  (`|SpawnActorFromClass` "/Game/Blueprints/Items/Weapons/FireArms/bp_MasterProjectile.bp_MasterProjectile_C" (`KismetMathLibrary.MakeTransform` (+ (`SceneComponent.GetSocketLocation` (`self.SkeletalMesh`) "Magazine") (`KismetMathLibrary.GreaterGreater_VectorRotator` (`self.Projectile Offset`) _returnvalue)) _returnvalue (0.25 0.03 0.03)) "AlwaysSpawn" "OverrideRootScale" null 1.0 1.0 null 10.0 null))

(fn `UserConstructionScript`)