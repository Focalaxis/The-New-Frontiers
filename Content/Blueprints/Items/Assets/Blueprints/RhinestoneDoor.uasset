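; RhinestoneDoor is a four-panel sliding door that opens when something overlaps its Box trigger and closes when an overlap ends.
; The Door_Open timeline plays forward on begin overlap and reverses on end overlap, with no filter on the overlapping actor.
; Its track drives lerps of each panel's relative location, sliding the left and right panels sideways and the top and bottom panels vertically apart.
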(event `self.Box.OnComponentBeginOverlap`
  (params (OverlappedComponent :type "PrimitiveComponent Object Reference") (OtherActor :type "Actor Object Reference") (OtherComp :type "PrimitiveComponent Object Reference") (OtherBodyIndex :type Integer) (bFromSweep :type Boolean) (SweepResult :type "HitResult Structure (by ref)"))
  (bind (_direction _newtrack_0) (`Timeline|Door_Open` :!label _label)
    (:`Update`
      (`SceneComponent.K2_SetRelativeLocation` (`self. R_Panel`) (`KismetMathLibrary.VLerp` (0.0 0.0 0.0) (20.0 0.0 0.0) _newtrack_0) false false)
      (`SceneComponent.K2_SetRelativeLocation` (`self.L_Panel`) (`KismetMathLibrary.VLerp` (0.0 0.0 0.0) (-20.0 0.0 0.0) _newtrack_0) false false)
      (`SceneComponent.K2_SetRelativeLocation` (`self.Top_Panel`) (`KismetMathLibrary.VLerp` (0.0 0.0 0.0) (0.0 0.0 70.0) _newtrack_0) false false)
      (`SceneComponent.K2_SetRelativeLocation` (`self.Bottom_Panel`) (`KismetMathLibrary.VLerp` (0.0 0.0 0.0) (0.0 0.0 -150.0) _newtrack_0) false false))))

(event `self.Box.OnComponentEndOverlap`
  (params (OverlappedComponent :type "PrimitiveComponent Object Reference") (OtherActor :type "Actor Object Reference") (OtherComp :type "PrimitiveComponent Object Reference") (OtherBodyIndex :type Integer))
  (goto _label :!via `Reverse`))

(fn `UserConstructionScript`)