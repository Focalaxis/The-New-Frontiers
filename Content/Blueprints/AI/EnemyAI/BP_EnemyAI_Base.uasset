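; Base enemy AI pawn with health, projectile firing, a health bar and a sight detection icon.
; BeginPlay caches both widgets and the Enemy_Ai controller, handing the pawn to the detection icon.
; AnyDamage lowers health and updates the bar, ragdolling the mesh only when health equals exactly zero.
; FireWeapon spawns Bp_MasterProjectile from an offset sphere, while Radius overlaps toggle health bar visibility around the cached FPS character.
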(event `self.ReceiveBeginPlay`
  (`|ExecutionSequence`
    (:`then_0`
      (bind _assight_detection_icon_wb (cast `/Game/UI/All_Levels/EnemyIcons/SightDetectionIcon_WB` (`WidgetComponent.GetUserWidgetObject` (`self.Detection`))))
      (set `self.As Sight Detection Icon WB` _assight_detection_icon_wb)
      (set `/Game/UI/All_Levels/EnemyIcons/SightDetectionIcon_WB.PawnOwner` self _assight_detection_icon_wb))
    (:`then_1`
      ;[1 1 1] Calls Health Bar Widget
      (bind _asenemy_health_wb (cast `/Game/UI/All_Levels/EnemyIcons/EnemyHealth_WB` (`WidgetComponent.GetWidget` (`self.HealthWidget`))))
      (bind _output_get (set `self.As Enemy Health WB` _asenemy_health_wb))
      (`/Game/UI/All_Levels/EnemyIcons/EnemyHealth_WB.UpdateHealth` _output_get (`self.Health`))
      ;[1 1 1] Sets Visibility at Begin Play
      (`Widget.SetVisibility` (`self.As Enemy Health WB`) "Hidden"))
    (:`then_2`
      (bind _asenemy_ai (cast `/Game/Blueprints/AI/EnemyAI/Enemy_Ai` (`AIBlueprintHelperLibrary.GetAIController` self)))
      (set `self.As Enemy Ai` _asenemy_ai))))

(event `FireWeapon`
  ;[1 1 1] Shoots gun
  (if (`self.IsAlive?`)
    (`self.SingleFire` (0.25 0.03 0.03) 10.0)))

(event `self.ReceiveAnyDamage`
  (params (Damage :type "Float (single-precision)") (DamageType :type "DamageType Object Reference") (InstigatedBy :type "Controller Object Reference") (DamageCauser :type "Actor Object Reference"))
  (bind _as_enemy_health_wb (`self.As Enemy Health WB`))
  ;[1 1 1] Takes damage
  (if (`self.IsAlive?`)
    (set `self.IsAlive` true)
    (bind _output_get (set `self.Health` (- (`self.Health`) Damage)))
    (if (== _output_get 0.0)
      (`self.Ragdoll`)
      (`/Game/UI/All_Levels/EnemyIcons/EnemyHealth_WB.UpdateHealth` (`self.As Enemy Health WB`) (`self.Health`))
      (`/Engine/EditorBlueprintResources/StandardMacros.IsValid` _as_enemy_health_wb
        (:`Is Valid`
          (`Widget.SetVisibility` _as_enemy_health_wb "Hidden")
          (if (`self.IsAlive?`)
            (`Widget.SetVisibility` (`self.As Sight Detection Icon WB`) "Hidden"))))
      (else
        (`/Game/UI/All_Levels/EnemyIcons/EnemyHealth_WB.UpdateHealth` (`self.As Enemy Health WB`) (/ (`self.Health`) (`self.Max Health`)))))
    (else
      (set `self.IsAlive` false))))

(event `Ragdoll`
  ;[1 1 1] Kills AI
  (`SkeletalMeshComponent.SetAllBodiesSimulatePhysics` (`self.Mesh`) true))

(event `self.Radius.OnComponentBeginOverlap`
  (params (OverlappedComponent :type "PrimitiveComponent Object Reference") (OtherActor :type "Actor Object Reference") (OtherComp :type "PrimitiveComponent Object Reference") (OtherBodyIndex :type Integer) (bFromSweep :type Boolean) (SweepResult :type "HitResult Structure (by ref)"))
  ;[1 1 1] Sets Visibility for Widget
  (`self.PlayerCast` OtherActor
    (:`then2`
      _)
    (:`then`
      _))
  (`Widget.SetVisibility` (`self.As Enemy Health WB`) "Visible"))

(event `self.Radius.OnComponentEndOverlap`
  (params (OverlappedComponent :type "PrimitiveComponent Object Reference") (OtherActor :type "Actor Object Reference") (OtherComp :type "PrimitiveComponent Object Reference") (OtherBodyIndex :type Integer))
  ;[1 1 1] Sets Visibility for Widget
  (if (== OtherActor (`self.As FPS Character`))
    (`Widget.SetVisibility` (`self.As Enemy Health WB`) "Hidden")))

(fn `GetProjectileSpawnLocation`
  (returns (Location :type "Vector Structure") (Rotation :type "Rotator Structure"))
  (bind _returnvalue (`SceneComponent.K2_GetComponentRotation` (`self.Sphere`)))
  (return (+ (`SceneComponent.K2_GetComponentLocation` (`self.Sphere`)) (`KismetMathLibrary.GreaterGreater_VectorRotator` (`self.ProjectileOffset`) _returnvalue)) _returnvalue))

(fn `IsAlive?`
  (returns (Alive :type Boolean))
  (return (> (`self.Health`) 0.0)))

(fn `SingleFire`
  (params (`Spawn Transform Scale` :type "Vector Structure" :default (0.25 0.03 0.03)) (`Base Damage` :type "Float (single-precision)" :default 0.34) (`Min Pitch` :type "Float (double-precision)" :default 1.0) (`Max Pitch` :type "Float (double-precision)" :default 1.0))
  (bind (_location _rotation) (`self.GetProjectileSpawnLocation`))
  (`|SpawnActorFromClass` "/Game/Blueprints/Items/FireArms/bp_MasterProjectile.bp_MasterProjectile_C" (`KismetMathLibrary.MakeTransform` _location _rotation `Spawn Transform Scale`) "AlwaysSpawn" "OverrideRootScale" null (`KismetMathLibrary.RandomFloatInRange` 0.4 0.6) (`KismetMathLibrary.RandomFloatInRange` `Min Pitch` `Max Pitch`) null `Base Damage` null))

(fn `UserConstructionScript`)