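; Base enemy Blueprint that takes weapon hits, tracks health and handles death.
; Damage is scaled by the hit physical material's DestructibleDamageThresholdScale, then subtracted from health.
; Each hit spawns a hit marker and randomly offset damage numbers flagging headshots by surface type, positioned using ImpactNormal as the location.
; Death ragdolls the mesh with a weapon-scaled impulse away from the player, plays a sound, removes the capsule and destroys the actor after a delay.
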(event `self.ReceiveBeginPlay`
  ;[1 0.4044 0] Get's reference to player
  (bind _asfps_character (cast `/Game/Blueprints/Character/FPS_Character` (`GameplayStatics.GetPlayerCharacter` 0)))
  (set `self.Player` _asfps_character))

(event `/Game/Blueprints/Interfaces/BPI_TakeDamage.EnemyTakeDamage`
  (params (WeaponStats :type "/Game/Blueprints/Items/Data/WeaponStats Structure") (HitResult :type "HitResult Structure"))
  (bind (_bblockinghit _binitialoverlap _time _distance _location _impactpoint _normal _impactnormal _physmat _hitactor _hitcomponent _hitbonename) (`GameplayStatics.BreakHitResult` HitResult))
  (if (not (`self.IsDead?`))
    (bind _calculateddamage (`self.CalculateDamage` (`.Damage_2_83DCFA9840A01BD66020149AB309A50F` (break `/Game/Blueprints/Items/Data/WeaponStats` WeaponStats)) HitResult))
    (bind _isdead_ (`self.HealthUpdate` _calculateddamage))
    (bind _output_get (set `self.IsDead?` _isdead_))
    (if _output_get
      (`self.EnemyDeath` _impactnormal _hitbonename)
      (`|ExecutionSequence`
        (:`then_0`
          (`KismetSystemLibrary.Delay` 60.0)
          (`self.K2_DestroyActor`))
        (:`then_1`
          (`self.DamageNumbers` _calculateddamage _impactnormal (`|EnumEquality` (`PhysicalMaterial.SurfaceType` _physmat) "SurfaceType1") :!label _label)
          (`/Engine/EditorBlueprintResources/StandardMacros.IsValid` null
            (:`Is Valid`
              (`Widget.RemoveFromParent` (`self.HitMarker Ref`)))
            (:`Is Not Valid`
              _))
          (bind _returnvalue (`|CreateWidget` "/Game/UI/All_Levels/PlayerHud/HitMarker.HitMarker_C" null (`self.IsDead?`)))
          (bind _output_get_2 (set `self.HitMarker Ref` _returnvalue))
          (`UserWidget.AddToViewport` _output_get_2 0)))
      (else
        (goto _label)))))

(event `self.DamageNumbers`
  (params (Damage :type "Float (double-precision)") (ImpactLocation :type "Vector Structure") (`IsHeadShot?` :type Boolean))
  (bind (_x _y) (`KismetMathLibrary.BreakVector2D` (`WidgetLayoutLibrary.ProjectWorldLocationToWidgetPosition` (`GameplayStatics.GetPlayerController` 0) ImpactLocation)))
  ;[0.8229 0.3403 0] Interface links Widget to Enemy Health and adds it to the screen
  (bind _returnvalue (`|CreateWidget` "/Game/UI/All_Levels/PlayerHud/DamageNumbers.DamageNumbers_C" null Damage `IsHeadShot?`))
  (`Widget.SetRenderTranslation` (`/Game/UI/All_Levels/PlayerHud/DamageNumbers.SizeBox` _returnvalue) (`KismetMathLibrary.MakeVector2D` (+ (+ _x -100.0) (`KismetMathLibrary.RandomFloatInRange` -25.0 150.0)) (+ (+ _y -100.0) (`KismetMathLibrary.RandomFloatInRange` 0.0 50.0))))
  (`UserWidget.AddToViewport` _returnvalue 0))

(fn `CalculateDamage`
  (params (Damage :type "Float (double-precision)") (HitResult :type "HitResult Structure"))
  (returns (CalculatedDamage :type "Float (double-precision)"))
  (locals (LocalDamage :type "Float (double-precision)"))
  (set `local.LocalDamage` Damage)
  (return (* (`local.LocalDamage`) (`PhysicalMaterial.DestructibleDamageThresholdScale` (`.PhysMat` (`GameplayStatics.BreakHitResult` HitResult))))))

(fn `EnemyDeath`
  (params (HitLocation :type "Vector Structure") (BoneName :type Name))
  (bind _player (`self.Player`))
  (`|ExecutionSequence`
    (:`then_0`
      ;[1 0.4044 0] Enabling Ragdoll Physics
      (`PrimitiveComponent.SetSimulatePhysics` (`self.Mesh`) true))
    (:`then_1`
      (`GameplayStatics.PlaySoundAtLocation` (`self.DeathLine`) (`self.K2_GetActorLocation`) (struct) 1.0 1.0 0.0 null null null null))
    (:`then_2`
      (`PrimitiveComponent.AddImpulseAtLocation` (`self.Mesh`) (* (`KismetMathLibrary.GetDirectionUnitVector` (`self.K2_GetActorLocation` _player) (`self.K2_GetActorLocation`)) (`/Game/Blueprints/Items/WeaponsV2/Weapons/WeaponBase.KillImpulse` (`/Game/Blueprints/Character/FPS_Character.CurrentWeapon` _player))) HitLocation BoneName)
      (`ActorComponent.K2_DestroyComponent` (`self.CapsuleComponent`)))))

(fn `HealthUpdate`
  (params (DamageApplied :type "Float (double-precision)"))
  (returns (`IsDead?` :type Boolean))
  (locals (`LocalIsDead?` :type Boolean))
  (`|ExecutionSequence`
    (:`then_0`
      (if (>= DamageApplied (`self.CurrentHealth`))
        (set `local.LocalIsDead?` true)
        (set `self.CurrentHealth` 0.0)
        (else
          (set `self.CurrentHealth` (- (`self.CurrentHealth`) DamageApplied)))))
    (:`then_1`
      (return (`local.LocalIsDead?`)))))

(fn `UserConstructionScript`)